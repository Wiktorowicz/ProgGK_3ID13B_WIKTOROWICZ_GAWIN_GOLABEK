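; BP_Trampoline is a parkour trampoline that launches the Ziomo1BP character straight up when it overlaps the Cube component.
; The overlap plays a sound at the cube and calls LaunchCharacter with both velocity overrides, replacing existing momentum with a fixed upward velocity.
; It also fires MoveTrampoline, which restarts a timeline that lerps the cube's relative Z downward to animate the bounce.
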(event OnComponentBeginOverlap(Cube)
  (params (OverlappedComponent :type Primitive%20Component%20Object%20Reference) (OtherActor :type Actor%20Object%20Reference) (OtherComp :type Primitive%20Component%20Object%20Reference) (OtherBodyIndex :type Integer) (bFromSweep :type Boolean) (SweepResult :type Hit%20Result%20Structure%20%28by%20ref%29))
  (bind _asziomo_1bp (Utilities|Casting|CastToZiomo1BP OtherActor))
  (CallFunction|MoveTrampoline)
  (Audio|PlaySoundatLocation "/Game/_AUDIO/wav/trampoline.trampoline" (Transformation|GetWorldLocation (Variables|Default|GetCube)) "0, 0, 0" 1.0 1.0 0.0 0 0 0 0)
  (Character|LaunchCharacter _asziomo_1bp "0.000000,0.000000,2000.000000" true true))

(event Custom|Move%20Trampoline
  (bind _alpha (Timeline|Trampoline%20Timeline PlayFromStart)
    (:Update
      (Transformation|SetRelativeLocation (Variables|Default|GetCube) (Math|Vector|MakeVector 0.0 0.0 (Math|Float|Lerp 0.0 -1e+02 _alpha)) false false))))

(fn ConstructionScript)