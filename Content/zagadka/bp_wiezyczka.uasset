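; Turret actor that spots the Ziomo1BP pawn and fires projectiles at it.
; Each PawnSensing sighting snaps the whole actor to face that pawn, with no other pawn class triggering a reaction.
; When the Strzelacczynie flag is on, a Delay precedes spawning Pocisk_bp1 at the Arrow component's transform.
; Sightings during that Delay still rotate the turret but queue no extra shots, so the Delay also limits fire rate.
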(event OnSeePawn(PawnSensing)
  (params (Pawn :type Pawn%20Object%20Reference))
  (Utilities|Casting|CastToZiomo1BP Pawn)
  (Transformation|SetActorRotation (Math|Rotator|FindLookatRotation (Transformation|GetActorLocation) (Transformation|GetActorLocation Pawn)))
  (if (Variables|Default|Getstrzelacczynie)
    (Utilities|FlowControl|Delay 2.0)
    (Game|SpawnActorfromClass "/Game/Nasze/pistol/pocisk_bp1.pocisk_bp1_C" (Transformation|GetWorldTransform (Variables|Default|GetArrow)) "Undefined" "MultiplyWithRoot" 0 0)))

(event EventBeginPlay)

(event Collision|EventActorBeginOverlap
  (params (OtherActor :type Actor%20Object%20Reference)))

(event EventTick
  (params (DeltaSeconds :type Float%20%28single-precision%29)))

(fn ConstructionScript)