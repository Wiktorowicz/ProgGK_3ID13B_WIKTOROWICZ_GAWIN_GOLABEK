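; Enemy AI character that chases the player once seen and hurts them on contact.
; PawnSensing sets a seen flag, never effectively cleared, and issues AI MoveTo, playing a rifle-shoot montage from its immediate output; Tick halts movement until then.
; Any Sphere overlap launches the player along a fixed world vector and applies IleHPZabiera damage, without checking the overlapping actor.
; The montage itself deals no damage.
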(event OnSeePawn(PawnSensing)
  (params (Pawn :type Pawn%20Object%20Reference))
  (Variables|Default|SetisSeeingPlayer? true)
  (CallFunction|FollowPlayer))

(event OnComponentBeginOverlap(Sphere)
  (params (OverlappedComponent :type Primitive%20Component%20Object%20Reference) (OtherActor :type Actor%20Object%20Reference) (OtherComp :type Primitive%20Component%20Object%20Reference) (OtherBodyIndex :type Integer) (bFromSweep :type Boolean) (SweepResult :type Hit%20Result%20Structure%20%28by%20ref%29))
  (bind _returnvalue (Game|GetPlayerCharacter 0))
  (Character|LaunchCharacter _returnvalue "1000.000000,0.000000,300.000000" false false)
  (Game|Damage|ApplyDamage _returnvalue (Math|Conversions|ToFloat(Integer) (Variables|Default|GetileHPZabiera)) 0 0))

(event Custom|FollowPlayer
  (Variables|Default|SetcanAttack? true)
  (if (Variables|Default|GetisSeeingPlayer?)
    (AI|AIMoveTo self "0, 0, 0" (Game|GetPlayerCharacter 0) 7e+01 false
      (:then
        (if (Variables|Default|GetcanAttack?)
          (Variables|Default|SetcanAttack? false)
          (bind _returnvalue (Animation|PlayAnimMontage "/Game/FirstPersonArms/Animations/FP_Rifle_Shoot_Montage.FP_Rifle_Shoot_Montage" 1.0 "None"))
          (Utilities|FlowControl|Delay _returnvalue)
          (Variables|Default|SetcanAttack? true))))
    (else
      (Variables|Default|SetisSeeingPlayer? false))))

(event EventBeginPlay)

(event Collision|EventActorBeginOverlap
  (params (OtherActor :type Actor%20Object%20Reference)))

(event EventTick
  (params (DeltaSeconds :type Float%20%28single-precision%29))
  (if (not (Variables|Default|GetisSeeingPlayer?))
    (Components|Movement|StopMovementImmediately (Variables|Character|GetCharacterMovement))))

(fn ConstructionScript)