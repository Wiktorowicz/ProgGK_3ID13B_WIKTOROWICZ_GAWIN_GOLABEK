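; BP_PuzzleDoor2 is a puzzle door that slides open and closed in response to BP_PuzzleButton2.
; On BeginPlay it finds the button through GetAllActorsOfClass and binds its Open and Close events to the button's dispatchers.
; Both events use MoveComponentTo to shift the static mesh along Y by opposite offsets from its current world location, passed as a relative target, with the same fixed rotation.
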(event Custom|Open
  (bind _staticmeshcomponent (Variables|Debug|GetStaticMeshComponent))
  (Components|MoveComponentTo _staticmeshcomponent (+ (Transformation|GetWorldLocation _staticmeshcomponent) "0.000000,-200.000000,0.000000") "0.000000,90.000000,0.000000" false false 0.2 false))

(event Custom|Close
  (bind _staticmeshcomponent (Variables|Debug|GetStaticMeshComponent))
  (Components|MoveComponentTo _staticmeshcomponent (- (Transformation|GetWorldLocation _staticmeshcomponent) "0.000000,-200.000000,0.000000") "0.000000,90.000000,0.000000" false false 0.2 false))

(event EventBeginPlay
  (bind _outactors (Actor|GetAllActorsOfClass "/Game/ButtonDoor/BP_PuzzleButton2.BP_PuzzleButton2_C"))
  (bind _output_get (Variables|Default|SetButton2Ref _outactors))
  (EventDispatchers|BindEventtoOpen2 _output_get (delegate Custom|Open))
  (EventDispatchers|BindEventtoClose2 _output_get (delegate Custom|Close)))

(fn ConstructionScript)