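; Disappearing platform that vanishes shortly after anything overlaps its trigger box, then returns.
; An overlap, gated by a DoOnce, brightens the cube's dynamic material and runs an opacity timeline while a parallel delay counts down to hiding the actor and disabling cube collision.
; After a second delay it restores visibility, collision and brightness, and a second opacity timeline resets the DoOnce from its first update, re-arming the trigger.
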(event OnComponentBeginOverlap(Box)
  (params (OverlappedComponent :type Primitive%20Component%20Object%20Reference) (OtherActor :type Actor%20Object%20Reference) (OtherComp :type Primitive%20Component%20Object%20Reference) (OtherBodyIndex :type Integer) (bFromSweep :type Boolean) (SweepResult :type Hit%20Result%20Structure%20%28by%20ref%29))
  ;[0.15 0.0805 0.00851 0.5] Znikajaca platforma
  (Utilities|FlowControl|DoOnce false :!label _label
    (:Completed
      (Rendering|Material|SetScalarParameterValue (Variables|Default|GetDynamic%20Material) "Bright" 3.0 :!class /Script/Engine.MaterialInstanceDynamic)
      (Utilities|FlowControl|Sequence
        (:then_0
          (bind _newtrack_0 (Timeline|Timeline PlayFromStart)
            (:Update
              (Rendering|Material|SetScalarParameterValue (Variables|Default|GetDynamic%20Material) "Opacity" _newtrack_0 :!class /Script/Engine.MaterialInstanceDynamic))))
        (:then_1
          (Utilities|FlowControl|Delay 1.0)
          (Rendering|SetActorHiddenInGame true)
          (Collision|SetCollisionEnabled (Variables|Default|GetCube) "NoCollision")
          (Utilities|FlowControl|Delay 2.0)
          (Rendering|SetActorHiddenInGame false)
          (Collision|SetCollisionEnabled (Variables|Default|GetCube) "QueryAndPhysics")
          (Rendering|Material|SetScalarParameterValue (Variables|Default|GetDynamic%20Material) "Bright" 0.0 :!class /Script/Engine.MaterialInstanceDynamic)
          (bind _newtrack_0_2 (Timeline|Timeline_0 PlayFromStart)
            (:Update
              (Rendering|Material|SetScalarParameterValue (Variables|Default|GetDynamic%20Material) "Opacity" _newtrack_0_2 :!class /Script/Engine.MaterialInstanceDynamic)
              (goto _label Reset))))))))

(event EventBeginPlay
  ;[0.15 0.0805 0.00851 0.5] Znikajaca platforma
  (bind _returnvalue (Rendering|Material|CreateDynamicMaterialInstance (Variables|Default|GetCube) 0 "/Game/Platforms/M_DisappearStage1.M_DisappearStage1" "None" :!class /Script/Engine.PrimitiveComponent))
  (bind _output_get (Variables|Default|SetDynamic%20Material _returnvalue))
  (Rendering|Material|SetScalarParameterValue _output_get "Bright" 0.0 :!class /Script/Engine.MaterialInstanceDynamic))

(fn ConstructionScript)