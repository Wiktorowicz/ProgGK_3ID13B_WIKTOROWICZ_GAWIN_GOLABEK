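; BP_Explosion is a destructible barrier that blows open when the player's PoziomStrzelnicy (shooting range level) equals 1.
; Tick polls Ziomo1BP, then applies a kinematic field and impulse to the geometry collection and spawns an explosion emitter.
; After a short Delay it plays the sound, sets the player's CzyOtwarta (is open) flag and makes the Box overlap pawns.
; Impulse and emitter repeat each tick until that flag is set.
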(event EventTick
  (params (DeltaSeconds :type Float%20%28single-precision%29))
  (bind _returnvalue (Transformation|GetActorLocation))
  (bind _asziomo_1bp (Utilities|Casting|CastToZiomo1BP (Game|GetPlayerCharacter 0)))
  (if (== (Variables|/Game/Ziomo1BP.Ziomo1BP_C|GetPoziomStrzelnicy _asziomo_1bp) 1)
    (if (not (Variables|/Game/Ziomo1BP.Ziomo1BP_C|GetczyOtwarta? _asziomo_1bp))
      (Class|GeometryCollectionComponent|ApplyKinematicField (Variables|Default|GetGeometryCollectionComponent) 0.0 "0, 0, 0")
      (Physics|AddImpulse (Variables|Default|GetGeometryCollectionComponent) "0.000000,5000.000000,1000.000000" "None" false)
      (Effects|SpawnEmitteratLocation "/Game/StarterContent/Particles/P_Explosion.P_Explosion" _returnvalue "0, 0, 0" "5.000000,5.000000,5.000000")
      (Utilities|FlowControl|Delay 0.2)
      (Audio|PlaySoundatLocation "/Game/StarterContent/Audio/Explosion01.Explosion01" _returnvalue "0, 0, 0" 1.0 1.0 0.0 0 0 0 0)
      (Variables|/Game/Ziomo1BP.Ziomo1BP_C|SetczyOtwarta? _asziomo_1bp true)
      (Collision|SetCollisionResponsetoChannel (Variables|Default|GetBox) "ECC_Pawn" "ECR_Overlap"))))

(fn ConstructionScript)