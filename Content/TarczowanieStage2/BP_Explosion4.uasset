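; BP_Explosion4 is a destructible obstacle that explodes and opens to pawns once the player reaches shooting-range level 6.
; Tick polls PoziomStrzelnicy on Ziomo1BP and, until Czyotwarta1 is set, applies a zero-valued kinematic field and impulse to its Geometry Collection.
; After a short delay it spawns a scaled-up explosion with sound, sets the flag and switches the Box's Pawn response to Overlap.
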(event EventTick
  (params (DeltaSeconds :type Float%20%28single-precision%29))
  (bind _returnvalue (Transformation|GetActorLocation))
  (bind _asziomo_1bp (Utilities|Casting|CastToZiomo1BP (Game|GetPlayerCharacter 0)))
  (if (== (Variables|/Game/Ziomo1BP.Ziomo1BP_C|GetPoziomStrzelnicy _asziomo_1bp) 6)
    (if (not (Variables|Default|Getczyotwarta1))
      (Class|GeometryCollectionComponent|ApplyKinematicField (Variables|Default|GetGeometryCollectionComponent) 0.0 "0, 0, 0")
      (Physics|AddImpulse (Variables|Default|GetGeometryCollectionComponent) "0, 0, 0" "None" false)
      (Utilities|FlowControl|Delay 0.32)
      (Effects|SpawnEmitteratLocation "/Game/StarterContent/Particles/P_Explosion.P_Explosion" _returnvalue "0, 0, 0" "10.000000,10.000000,10.000000")
      (Audio|PlaySoundatLocation "/Game/StarterContent/Audio/Explosion01.Explosion01" _returnvalue "0, 0, 0" 1.2 1.0 0.0 0 0 0 0)
      (Variables|Default|Setczyotwarta1 true)
      (Collision|SetCollisionResponsetoChannel (Variables|Default|GetBox) "ECC_Pawn" "ECR_Overlap"))))

(fn ConstructionScript)