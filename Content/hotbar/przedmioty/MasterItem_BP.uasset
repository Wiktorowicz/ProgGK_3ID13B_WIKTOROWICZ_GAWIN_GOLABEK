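; MasterItem_BP is a pickup item actor, apparently the base for hotbar items, that the player collects by pressing F.
; Overlapping its Collision component with a Ziomo1BP stores that character and enables player 0's input on the item; ending any overlap disables it.
; Pressing F passes the item's ItemInfo to the character's PickItems function, then destroys the actor.
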(event OnComponentBeginOverlap(collision)
  (params (OverlappedComponent :type Primitive%20Component%20Object%20Reference) (OtherActor :type Actor%20Object%20Reference) (OtherComp :type Primitive%20Component%20Object%20Reference) (OtherBodyIndex :type Integer) (bFromSweep :type Boolean) (SweepResult :type Hit%20Result%20Structure%20%28by%20ref%29))
  (bind _asziomo_1bp (Utilities|Casting|CastToZiomo1BP OtherActor))
  (Variables|Default|SetcharacterCast _asziomo_1bp)
  (Input|EnableInput (Game|GetPlayerController 0)))

(event OnComponentEndOverlap(collision)
  (params (OverlappedComponent :type Primitive%20Component%20Object%20Reference) (OtherActor :type Actor%20Object%20Reference) (OtherComp :type Primitive%20Component%20Object%20Reference) (OtherBodyIndex :type Integer))
  (Input|DisableInput (Game|GetPlayerController 0)))

(event Input|KeyboardEvents|F
  (params (Key :type Key%20Structure :default "None"))
  (:Pressed
    (Default|PickItems (Variables|Default|GetcharacterCast) (Variables|Default|GetItemInfo))
    (Actor|DestroyActor)))

(fn ConstructionScript)